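; Game mode for LeaveMeAlone that runs the match countdown and shows the two end-of-game screens.
; A looping one-second timer started on BeginPlay decrements GameTime, then at zero clears itself and shows WBP_GameEnd.
; A separate RecieverFunction event, with no caller in this graph, shows WBP_GameOver.
; Both endings switch the first player to UI-only input with a visible cursor.
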(event `self.ReceiveBeginPlay`
  (bind _returnvalue (`KismetSystemLibrary.K2_SetTimerDelegate` (delegate `CustomEvent`) 1.0 true))
  (set `self.GameTimerHandle` _returnvalue))

(event `CustomEvent`
  (bind _returnvalue (`GameplayStatics.GetPlayerController` 0))
  (bind _output_get (set `self.GameTime` (- (`self.GameTime`) 1)))
  (if (== _output_get 0)
    (`KismetSystemLibrary.K2_ClearAndInvalidateTimerHandle` (`self.GameTimerHandle`))
    (bind _returnvalue_2 (`|CreateWidget` "/Game/LeaveMeAlone/Widgets/UI/WBP_GameEnd.WBP_GameEnd_C"))
    (bind _output_get_2 (set `self.GameEnd` _returnvalue_2))
    (`UserWidget.AddToViewport` _output_get_2 0)
    (`WidgetBlueprintLibrary.SetInputMode_UIOnlyEx` _returnvalue _output_get_2)
    (set `PlayerController.bShowMouseCursor` true _returnvalue)))

(event `/Game/LeaveMeAlone/Core/Interfaces/BP_Interface.Reciever Function`
  (bind _returnvalue (`GameplayStatics.GetPlayerController` 0))
  (bind _returnvalue_2 (`|CreateWidget` "/Game/LeaveMeAlone/Widgets/UI/WBP_GameOver.WBP_GameOver_C"))
  (bind _output_get (set `self.GameOver` _returnvalue_2))
  (`UserWidget.AddToViewport` _output_get 0)
  (`WidgetBlueprintLibrary.SetInputMode_UIOnlyEx` _returnvalue null)
  (set `PlayerController.bShowMouseCursor` true _returnvalue))

(fn `UserConstructionScript`)